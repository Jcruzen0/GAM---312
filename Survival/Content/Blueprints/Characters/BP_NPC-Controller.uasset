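; AI controller that makes its possessed NPC wander between random navigable points near its current location.
; Tick watches the NewDestination flag, waits a random short delay, then calls Wander and clears the flag.
; Wander picks a point within a fixed radius and runs AIMoveTo, re-arming the flag only on success, so a failed move does not trigger another.
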(event Custom|Wander
  (bind _returnvalue (Pawn|GetControlledPawn))
  (bind _randomlocation (Class|NavigationSystemV1|GetRandomLocationinNavigableRadius (Transformation|GetActorLocation _returnvalue) 6e+02 0 0))
  (AI|AIMoveTo _returnvalue _randomlocation 0 5.0 false
    (:OnSuccess
      (Variables|Default|SetnewDestination true))))

(event EventBeginPlay)

(event EventTick
  (params (DeltaSeconds :type Float%20%28single-precision%29))
  (if (Variables|Default|GetnewDestination)
    (Utilities|FlowControl|Delay (Math|Random|RandomFloat))
    (CallFunction|Wander)
    (Variables|Default|SetnewDestination false)))

(fn ConstructionScript)